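; BP_Alisson_Board_Counting is a counting board Blueprint that relays a count to its WDG_Cube_Counter widget component.
; GraysonHelp casts the component's widget, and when the input equals seven it calls FoundBoxes and plays a coin sound at the world origin.
; Any other input updates the displayed amount and calls LostBoxes.
; The construction script only runs the parent's.
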(fn ConstructionScript
  (|CallParentFunction))

(fn GraysonHelp
  (params (NewInput :type Integer))
  (bind _aswdg_cube_counter (Utilities|Casting|CastToWDG_Cube_Counter (UserInterface|GetUserWidgetObject (Variables|Default|GetComp_Widget))))
  (if (== NewInput 7)
    (bind _aswdg_cube_counter_2 (Utilities|Casting|CastToWDG_Cube_Counter (UserInterface|GetUserWidgetObject (Variables|Default|GetComp_Widget))))
    (Default|FoundBoxes _aswdg_cube_counter_2)
    (Audio|PlaySoundatLocation "/Game/Interface_And_Item_Sounds/Cues/Coins_13_Cue.Coins_13_Cue" "0, 0, 0" "0, 0, 0" 1.0 1.0 0.0 0 0 0)
    (else
      (Default|UpdateAmount _aswdg_cube_counter NewInput)
      (Default|LostBoxes _aswdg_cube_counter))))