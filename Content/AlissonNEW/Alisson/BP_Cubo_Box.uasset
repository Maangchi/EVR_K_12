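; BP_Cubo_Box is a trigger box that counts the BP_Cubo actors inside it and shows the count on screen.
; On BeginPlay it creates a WDG_Cube_Counter widget, stores the reference and adds it to the viewport.
; Each begin overlap on CollisionBox passes the current number of overlapping cubes to the widget.
; End overlap only prints a debug string, so the counter does not update when cubes leave.
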(event OnComponentBeginOverlap(CollisionBox)
  (params (OverlappedComponent :type Primitive%20Component%20Object%20Reference) (OtherActor :type Actor%20Object%20Reference) (OtherComp :type Primitive%20Component%20Object%20Reference) (OtherBodyIndex :type Integer) (bFromSweep :type Boolean) (SweepResult :type Hit%20Result%20Structure%20%28by%20ref%29))
  (Default|UpdateAmount (Variables|Default|GetReference%20Counter) (Utilities|Array|Length (Collision|GetOverlappingActors (Variables|Default|GetCollisionBox) "/Game/AlissonNEW/Alisson/BP_Cubo.BP_Cubo_C" :!class /Script/Engine.PrimitiveComponent))))

(event OnComponentEndOverlap(CollisionBox)
  (params (OverlappedComponent :type Primitive%20Component%20Object%20Reference) (OtherActor :type Actor%20Object%20Reference) (OtherComp :type Primitive%20Component%20Object%20Reference) (OtherBodyIndex :type Integer))
  (Development|PrintString "Hello"))

(event EventBeginPlay
  (bind _returnvalue (UserInterface|CreateWidget "/Game/AlissonNEW/Alisson/WDG_Cube_Counter.WDG_Cube_Counter_C"))
  (bind _output_get (Variables|Default|SetReference%20Counter _returnvalue))
  (UserInterface|Viewport|AddtoViewport _output_get 0))

(fn ConstructionScript)