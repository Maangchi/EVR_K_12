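; BP_DoorPortal is a door portal that sends the player to another level.
; When a pawn overlaps its TriggerBox, it stores its DoorID on the main game instance, then opens the level named by its Destination enum.
; On BeginPlay it sets the DestinationName text to the DoorID rather than the destination level.
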(event OnComponentBeginOverlap(TriggerBox)
  (params (OverlappedComponent :type Primitive%20Component%20Object%20Reference) (OtherActor :type Actor%20Object%20Reference) (OtherComp :type Primitive%20Component%20Object%20Reference) (OtherBodyIndex :type Integer) (bFromSweep :type Boolean) (SweepResult :type Hit%20Result%20Structure%20%28by%20ref%29))
  (bind _aspawn (Utilities|Casting|CastToPawn OtherActor))
  (bind _gameinstance (CallFunction|GetMainGameInstance _aspawn))
  (Variables|/Game/AFCore/Blueprints/Game/BP_GameInstance_Main.BP_GameInstance_Main_C|SetDoorID _gameinstance (Variables|Default|GetDoorID))
  (Game|OpenLevel(byName) (Utilities|String|StringToName (Utilities|String|EnumtoString (Variables|Default|GetDestination)))))

(event EventBeginPlay
  (Rendering|Components|TextRender|SetText (Variables|Default|GetDestination%20Name) (Utilities|Text|MakeLiteralText (Utilities|Text|ToText(Name) (Utilities|String|StringToName (Utilities|String|ToString(Name) (Variables|Default|GetDoorID)))))))

(event Collision|EventActorBeginOverlap
  (params (OtherActor :type Actor%20Object%20Reference)))

(event EventTick
  (params (DeltaSeconds :type Float%20%28single-precision%29)))

(fn ConstructionScript)