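; BP_Door_Alchemy is a double door whose left and right leaves open automatically for pawns.
; Each leaf has its own trigger: pawn overlap begin swings it open, overlap end swings it closed.
; Separate open and close timelines per leaf scale a SlideOpen value by that side's open amount to set relative Z rotation.
; Timelines always restart from an endpoint: opening plays from start, closing reverses from end.
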(event OnComponentBeginOverlap(DoorLeft_Trigger)
  (params (OverlappedComponent :type Primitive%20Component%20Object%20Reference) (OtherActor :type Actor%20Object%20Reference) (OtherComp :type Primitive%20Component%20Object%20Reference) (OtherBodyIndex :type Integer) (bFromSweep :type Boolean) (SweepResult :type Hit%20Result%20Structure%20%28by%20ref%29))
  (Utilities|Casting|CastToPawn OtherActor)
  (bind _slide_open (Timeline|Rotate_Open_Left PlayFromStart)
    (:Update
      (Utilities|SetRelativeRotationZ (Variables|Default|GetDoorLeft) (* _slide_open (Variables|Default|GetOpen%20Left%20Amount)) false false))))

(event OnComponentEndOverlap(DoorLeft_Trigger)
  (params (OverlappedComponent :type Primitive%20Component%20Object%20Reference) (OtherActor :type Actor%20Object%20Reference) (OtherComp :type Primitive%20Component%20Object%20Reference) (OtherBodyIndex :type Integer))
  (Utilities|Casting|CastToPawn OtherActor)
  (bind _slide_open (Timeline|Rotate_Close_Left ReverseFromEnd)
    (:Update
      (Utilities|SetRelativeRotationZ (Variables|Default|GetDoorLeft) (* _slide_open (Variables|Default|GetOpen%20Left%20Amount)) false false))))

(event OnComponentBeginOverlap(DoorRight_Trigger)
  (params (OverlappedComponent :type Primitive%20Component%20Object%20Reference) (OtherActor :type Actor%20Object%20Reference) (OtherComp :type Primitive%20Component%20Object%20Reference) (OtherBodyIndex :type Integer) (bFromSweep :type Boolean) (SweepResult :type Hit%20Result%20Structure%20%28by%20ref%29))
  (Utilities|Casting|CastToPawn OtherActor)
  (bind _slide_open (Timeline|Rotate_Open_Right PlayFromStart)
    (:Update
      (Utilities|SetRelativeRotationZ (Variables|Default|GetDoorRight) (* _slide_open (Variables|Default|GetOpen%20Right%20Amount)) false false))))

(event OnComponentEndOverlap(DoorRight_Trigger)
  (params (OverlappedComponent :type Primitive%20Component%20Object%20Reference) (OtherActor :type Actor%20Object%20Reference) (OtherComp :type Primitive%20Component%20Object%20Reference) (OtherBodyIndex :type Integer))
  (Utilities|Casting|CastToPawn OtherActor)
  (bind _slide_open (Timeline|Rotate_Close_Right ReverseFromEnd)
    (:Update
      (Utilities|SetRelativeRotationZ (Variables|Default|GetDoorRight) (* _slide_open (Variables|Default|GetOpen%20Right%20Amount)) false false))))

(event Collision|EventActorBeginOverlap
  (params (OtherActor :type Actor%20Object%20Reference)))

(event EventTick
  (params (DeltaSeconds :type Float%20%28single-precision%29)))

(fn ConstructionScript)