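; BP_UserPass_Runtime loads student records, presumably login credentials, from a public Google Sheet at runtime.
; On BeginPlay it builds the download link from SheetURL and fetches the sheet as CSV.
; The completion callback validates the download with empty backup paths, then fills the StudentsStruct array from the CSV.
; A failed array update prints an error, while a failed validation is silent.
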(event Custom|Execute!
  (params (CallbackInfo :type Runtime%20Data%20Table%20Callback%20Info%20Structure))
  (bind (_outcsvinfo _outresultcode _returnvalue) (Class|RuntimeDataTableObject|ValidateGoogleSheetsDownloadandLoadBackupifNeeded CallbackInfo))
  (if _returnvalue
    (Variables|Default|SetCSV_Info_Result _outcsvinfo)
    (bind _successful (Class|RuntimeDataTableObject|UpdateArrayfromCsvInfo (Variables|Default|GetStudentsStruct) (Variables|Default|GetCSV_Info_Result)))
    (if (not _successful)
      (Development|PrintString "Failed Update Array From Csv Info"))))

(event EventBeginPlay
  (Class|RuntimeDataTableObject|BuildGoogleSheetDownloadLinkandGetasCsv :CallOnComplete (delegate Custom|Execute!) :InSheetURL (Variables|Default|GetSheetURL) :bSheetIsPublic true))

(fn ConstructionScript)