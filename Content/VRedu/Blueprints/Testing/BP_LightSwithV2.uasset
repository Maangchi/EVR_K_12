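; BP_LightSwithV2 is a light switch Blueprint that controls the visibility and brightness of the lights in its Lights array.
; On BeginPlay it passes itself to the Widget_LightSwitch in its widget component, giving the UI a reference to the switch.
; Its on/off event sets each light's root component hidden from the boolean input (true hides).
; DecBrightness and IncBrightness both set point light intensity directly to the supplied value.
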(event EventTurnLightsOn/Off
  (params (TurnLightOn/Off2 :type Boolean))
  (for _array_element (Variables|Default|GetLights)
    (Development|SetHiddeninGame (Variables|/Script/Engine.Actor|GetRootComponent _array_element) TurnLightOn/Off2 false)))

(event EventBeginPlay
  (bind _aswidget_light_switch (Utilities|Casting|CastToWidget_LightSwitch (UserInterface|GetUserWidgetObject (Variables|Default|GetComp_Widget))))
  (Variables|/Game/VRedu/Blueprints/UI/Widgets/Widget_LightSwitch.Widget_LightSwitch_C|SetBP_LightSwitch _aswidget_light_switch self))

(event EventDecBrightness
  (params (DecreaseBrightness :type Float%20%28single-precision%29))
  (for _array_element (Variables|Default|GetLights)
    (Rendering|Components|Light|SetIntensity (Variables|/Script/Engine.PointLight|GetPointLightComponent _array_element) DecreaseBrightness)))

(event EventIncBrightness
  (params (IncreaseBrightness :type Float%20%28single-precision%29))
  (for _array_element (Variables|Default|GetLights)
    (Rendering|Components|Light|SetIntensity (Variables|/Script/Engine.PointLight|GetPointLightComponent _array_element) IncreaseBrightness)))

(fn ConstructionScript
  (|CallParentFunction))